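; BP_SplineLayoutTool is a level layout actor that places copies of a chosen mesh along a spline.
; Its Construction Script spaces instanced static mesh instances by the mesh's bounding-box X size plus an offset, filling the spline's length.
; Each instance takes pitch and yaw from the spline tangent, with yaw turned 90 degrees, and roll from the spline rotation's pitch.
; The event graph has no runtime logic.
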(event EventBeginPlay)

(event Collision|EventActorBeginOverlap
  (params (OtherActor :type Actor%20Object%20Reference)))

(event EventTick
  (params (DeltaSeconds :type Float%20%28single-precision%29)))

(fn ConstructionScript
  (bind _placedmesh (Variables|Default|GetPlacedMesh))
  (bind _spline (Variables|Default|GetSpline))
  (bind _returnvalue (StaticMesh|GetBoundingBox _placedmesh))
  (bind (_min _max) (Utilities|Struct|BreakBox _returnvalue))
  (Components|StaticMesh|SetStaticMesh (Variables|Default|GetInstancedStaticMesh) (Variables|Default|GetPlacedMesh))
  (bind _output_get (Variables|Default|SetSpacing (+ (.X (Math|Vector|BreakVector (- _max _min))) (Variables|Default|GetOffset))))
  (bind _output_get_2 (LocalVariables|SetNumberOfInstances (Math|Float|Floor (/ (Spline|GetSplineLength (Variables|Default|GetSpline)) _output_get))))
  (for _index (range 0 _output_get_2)
    (Components|InstancedStaticMesh|AddInstance (Variables|Default|GetInstancedStaticMesh) (Math|Transform|MakeTransform (Spline|GetLocationatDistanceAlongSpline _spline (* _index (Variables|Default|GetSpacing)) "Local") (Math|Rotator|MakeRotator (.pitch (Spline|GetRotationatDistanceAlongSpline _spline (* _index (Variables|Default|GetSpacing)) "Local")) (.pitch (Math|Conversions|RotationFromXVector (Spline|GetTangentatDistanceAlongSpline _spline (* _index (Variables|Default|GetSpacing)) "Local"))) (+ (.yaw (Math|Conversions|RotationFromXVector (Spline|GetTangentatDistanceAlongSpline _spline (* _index (Variables|Default|GetSpacing)) "Local"))) 9e+01))) false)))