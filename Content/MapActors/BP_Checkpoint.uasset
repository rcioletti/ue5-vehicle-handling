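; BP_Checkpoint is a lap line actor that counts race car laps, saves best lap times and ends the race.
; When a RaceCarPawn leaves the Cube overlap, it increments the lap, records the lap time and clears the timer.
; For pawns with a VehiclePlayerController, it saves any improved best time through RaceGameInstance.
; Once laps exceed SPRaceGameMode's limit, it calls EndRace on the controller and brakes the car.
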(event OnComponentEndOverlap(Cube)
  (params (OverlappedComponent :type Primitive%20Component%20Object%20Reference) (OtherActor :type Actor%20Object%20Reference) (OtherComp :type Primitive%20Component%20Object%20Reference) (OtherBodyIndex :type Integer))
  (bind _asrace_car_pawn (Utilities|Casting|CastToRaceCarPawn OtherActor))
  (bind _output_get (Variables|Default|SetAs%20Race%20Car%20Pawn _asrace_car_pawn))
  (Development|PrintString (Utilities|String|ToString(Integer) (Variables|/Script/Handling.RaceCarPawn|GetCurrentLap _output_get)))
  (Variables|/Script/Handling.RaceCarPawn|SetCurrentLap _output_get (+ (Variables|/Script/Handling.RaceCarPawn|GetCurrentLap _output_get) 1))
  (Utilities|Array|Add (Variables|/Script/Handling.RaceCarPawn|GetLapTimes (Variables|Default|GetAs%20Race%20Car%20Pawn)) (Variables|/Script/Handling.RaceCarPawn|GetTimeCounter (Variables|Default|GetAs%20Race%20Car%20Pawn)))
  (Class|RaceCarPawn|ClearTimer (Variables|Default|GetAs%20Race%20Car%20Pawn))
  (bind _asvehicle_player_controller (Utilities|Casting|CastToVehiclePlayerController (Pawn|GetController _asrace_car_pawn)))
  (Variables|Default|SetAs%20Vehicle%20Player%20Controller _asvehicle_player_controller)
  (CallFunction|SaveGame)
  (bind _assprace_game_mode (Utilities|Casting|CastToSPRaceGameMode (Game|GetGameMode)))
  (if (> (Variables|/Script/Handling.RaceCarPawn|GetCurrentLap (Variables|Default|GetAs%20Race%20Car%20Pawn)) (Variables|/Script/Handling.SPRaceGameMode|GetGameLaps _assprace_game_mode))
    (Utilities|IsValid (Variables|Default|GetAs%20Vehicle%20Player%20Controller)
      (:Is%20Valid
        (Default|EndRace (Variables|Default|GetAs%20Vehicle%20Player%20Controller))
        (Class|ChaosVehicleMovementComponent|SetThrottleInput (Variables|/Script/ChaosVehicles.WheeledVehiclePawn|GetVehicleMovementComponent (Variables|Default|GetAs%20Race%20Car%20Pawn)) 0.0)
        (Class|ChaosVehicleMovementComponent|SetBrakeInput (Variables|/Script/ChaosVehicles.WheeledVehiclePawn|GetVehicleMovementComponent (Variables|Default|GetAs%20Race%20Car%20Pawn)) 1.0)))))

(event EventBeginPlay)

(event Collision|EventActorBeginOverlap
  (params (OtherActor :type Actor%20Object%20Reference)))

(event EventTick
  (params (DeltaSeconds :type Float%20%28single-precision%29)))

(fn ConstructionScript)

(fn SaveGame
  (bind _returnvalue (Class|RaceCarPawn|GetCurrentBestTime (Variables|Default|GetAs%20Race%20Car%20Pawn)))
  (bind _asrace_game_instance (Utilities|Casting|CastToRaceGameInstance (Game|GetGameInstance)))
  (if (> (Variables|/Script/Handling.RaceSaveGame|GetBestLapTime (Variables|/Script/Handling.RaceGameInstance|GetSaveGameObject _asrace_game_instance)) _returnvalue)
    (Variables|/Script/Handling.RaceSaveGame|SetBestLapTime (Variables|/Script/Handling.RaceGameInstance|GetSaveGameObject _asrace_game_instance) _returnvalue)
    (Class|RaceGameInstance|SaveGame _asrace_game_instance)))