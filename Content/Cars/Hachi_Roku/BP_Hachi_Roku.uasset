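; Player-drivable Hachi Roku race car on Chaos vehicle physics, with nitrous, manual shifting, brake lights, pause and reset to the nearest spline point.
; Enhanced Input drives the movement component, while BeginPlay applies saved paint from the game instance.
; Releasing throttle triggers drift by changing wheel friction and slip multipliers; pressing it restores grip.
; Tick recharges nitrous, damps airborne rotation, recentres the camera, scales FOV with speed and feeds engine audio.
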(event OnComponentBeginOverlap(Box)
  (params (OverlappedComponent :type Primitive%20Component%20Object%20Reference) (OtherActor :type Actor%20Object%20Reference) (OtherComp :type Primitive%20Component%20Object%20Reference) (OtherBodyIndex :type Integer) (bFromSweep :type Boolean) (SweepResult :type Hit%20Result%20Structure%20%28by%20ref%29))
  (Utilities|FlowControl|DoOnce false :!label _label
    (:Completed
      (Audio|PlaySoundatLocation "/Game/Sound/Toyota_Trueno/Sounds/tyre_explosion__5163cf31-54eb-4a39-9214-b4ebefad26a2_.tyre_explosion__5163cf31-54eb-4a39-9214-b4ebefad26a2_" "0, 0, 0" "0, 0, 0" 0.3 1.0 0.0 0 0 0 0)
      (Utilities|FlowControl|Delay 0.3)
      (goto _label Reset))))

(event Custom|InterpsToOriginalRotation
  (Transformation|SetRelativeRotation (Variables|Default|GetSpringArm) (Math|Rotator|MakeRotator 0.0 0.0 (Math|Interpolation|FInterpTo (.yaw (Variables|/Script/Engine.SceneComponent|GetRelativeRotation (Variables|Default|GetSpringArm))) 0.0 (Utilities|Time|GetWorldDeltaSeconds) 1.0)) false false) ; Reset camera to original angle
)

(event Custom|Drift
  (bind _chaos_wheeled_vehicle_movement_component (Variables|Default|GetChaos%20Wheeled%20Vehicle%20Movement%20Component))
  (Class|ChaosWheeledVehicleMovementComponent|SetWheelFrictionMultiplier (Variables|Default|GetChaos%20Wheeled%20Vehicle%20Movement%20Component) 2 0.5)
  (Class|ChaosWheeledVehicleMovementComponent|SetWheelFrictionMultiplier _chaos_wheeled_vehicle_movement_component 3 0.5)
  (Class|ChaosWheeledVehicleMovementComponent|SetWheelSlipGraphMultiplier _chaos_wheeled_vehicle_movement_component 0 0.75)
  (Class|ChaosWheeledVehicleMovementComponent|SetWheelSlipGraphMultiplier _chaos_wheeled_vehicle_movement_component 1 0.75))

(event Custom|Grip
  (bind _chaos_wheeled_vehicle_movement_component (Variables|Default|GetChaos%20Wheeled%20Vehicle%20Movement%20Component))
  (Class|ChaosWheeledVehicleMovementComponent|SetWheelFrictionMultiplier (Variables|Default|GetChaos%20Wheeled%20Vehicle%20Movement%20Component) 2 3.0)
  (Class|ChaosWheeledVehicleMovementComponent|SetWheelFrictionMultiplier _chaos_wheeled_vehicle_movement_component 3 3.0)
  (Class|ChaosWheeledVehicleMovementComponent|SetWheelSlipGraphMultiplier _chaos_wheeled_vehicle_movement_component 0 1.0)
  (Class|ChaosWheeledVehicleMovementComponent|SetWheelSlipGraphMultiplier _chaos_wheeled_vehicle_movement_component 1 1.0))

(event Custom|ChargeNitrous
  (if (<= (Variables|Default|GetNitrousContent) 1.0)
    (Variables|Default|SetNitrousContent (+ (Variables|Default|GetNitrousContent) 0.0005))))

(event Input|EnhancedActionEvents|EnhancedInputActionIA_Throttle
  (params (ActionValue :type Float%20%28double-precision%29) (ElapsedSeconds :type Float%20%28double-precision%29) (TriggeredSeconds :type Float%20%28double-precision%29) (InputAction :type Input%20Action%20Object%20Reference :default "/Game/Input/Actions/IA_Throttle.IA_Throttle"))
  (bind _vehiclemovementcomponent (Variables|Default|GetVehicleMovementComponent))
  (:Triggered
    (Class|ChaosVehicleMovementComponent|SetThrottleInput _vehiclemovementcomponent ActionValue)
    (Camera|PlayWorldCameraShake "/Game/Cars/CarCameraShake.CarCameraShake_C" (Transformation|GetWorldLocation (Variables|Default|GetCamera)) 0.0 5e+02))
  (:Started
    (CallFunction|Grip))
  (:Completed
    (CallFunction|Drift)
    (Class|ChaosVehicleMovementComponent|SetThrottleInput _vehiclemovementcomponent ActionValue)))

(event Input|EnhancedActionEvents|EnhancedInputActionIA_Brake
  (params (ActionValue :type Float%20%28double-precision%29) (ElapsedSeconds :type Float%20%28double-precision%29) (TriggeredSeconds :type Float%20%28double-precision%29) (InputAction :type Input%20Action%20Object%20Reference :default "/Game/Input/Actions/IA_Brake.IA_Brake"))
  (bind _vehiclemovementcomponent (Variables|Default|GetVehicleMovementComponent))
  (:Triggered
    (Class|ChaosVehicleMovementComponent|SetBrakeInput _vehiclemovementcomponent ActionValue)
    (CallFunction|BrakeLights true))
  (:Completed
    (Class|ChaosVehicleMovementComponent|SetBrakeInput _vehiclemovementcomponent 0.0)
    (CallFunction|BrakeLights false)))

(event Input|EnhancedActionEvents|EnhancedInputActionIA_GearUp
  (params (ActionValue :type Float%20%28double-precision%29) (ElapsedSeconds :type Float%20%28double-precision%29) (TriggeredSeconds :type Float%20%28double-precision%29) (InputAction :type Input%20Action%20Object%20Reference :default "/Game/Input/Actions/IA_GearUp.IA_GearUp"))
  (bind _chaos_wheeled_vehicle_movement_component (Variables|Default|GetChaos%20Wheeled%20Vehicle%20Movement%20Component))
  (:Started
    (Class|ChaosVehicleMovementComponent|SetTargetGear _chaos_wheeled_vehicle_movement_component (+ (Class|ChaosVehicleMovementComponent|GetTargetGear _chaos_wheeled_vehicle_movement_component) 1) true)))

(event Input|EnhancedActionEvents|EnhancedInputActionIA_Handbrake
  (params (ActionValue :type Boolean) (ElapsedSeconds :type Float%20%28double-precision%29) (TriggeredSeconds :type Float%20%28double-precision%29) (InputAction :type Input%20Action%20Object%20Reference :default "/Game/Input/Actions/IA_Handbrake.IA_Handbrake"))
  (:Triggered
    (Class|ChaosVehicleMovementComponent|SetHandbrakeInput (Variables|Default|GetVehicleMovementComponent) ActionValue :!label _label))
  (:Completed
    (goto _label)))

(event Input|EnhancedActionEvents|EnhancedInputActionIA_LookAround
  (params (ActionValue :type Float%20%28double-precision%29) (ElapsedSeconds :type Float%20%28double-precision%29) (TriggeredSeconds :type Float%20%28double-precision%29) (InputAction :type Input%20Action%20Object%20Reference :default "/Game/Input/Actions/IA_LookAround.IA_LookAround"))
  (Transformation|AddLocalRotation (Variables|Default|GetSpringArm) (Math|Rotator|MakeRotator 0.0 0.0 ActionValue) false false) ; Rotate camera around the vehicle
)

(event Input|EnhancedActionEvents|EnhancedInputActionIA_Nitrous
  (params (ActionValue :type Boolean) (ElapsedSeconds :type Float%20%28double-precision%29) (TriggeredSeconds :type Float%20%28double-precision%29) (InputAction :type Input%20Action%20Object%20Reference :default "/Game/Input/Actions/IA_Nitrous.IA_Nitrous"))
  (bind _mesh (Variables|Character|GetMesh))
  (:Triggered
    (if (> (Variables|Default|GetNitrousContent) 0.0)
      (Variables|Default|SetNitrousContent (- (Variables|Default|GetNitrousContent) 0.01))
      (Physics|AddImpulse _mesh (* (Math|Vector|GetForwardVector _mesh) 2e+01) "None" true)
      (else
        (Audio|Parameter|SetFloatParameter (Variables|Default|GetNitrous%20Audio) "Volume" 0.0 :!class /Script/Engine.AudioComponent :!label _label))))
  (:Started
    (Audio|Parameter|SetFloatParameter (Variables|Default|GetNitrous%20Audio) "Volume" 1.0 :!class /Script/Engine.AudioComponent)
    (Effects|SpawnEmitterAttached (Variables|Default|GetExhaustPopParticle) (Variables|Default|GetExhaustAudioComponent) "None" "0, 0, 0" "0, 0, 0" "0.300000,0.300000,0.300000" "SnapToTargetIncludingScale" true "AutoRelease"))
  (:Completed
    (goto _label)))

(event Input|EnhancedActionEvents|EnhancedInputActionIA_Reset
  (params (ActionValue :type Boolean) (ElapsedSeconds :type Float%20%28double-precision%29) (TriggeredSeconds :type Float%20%28double-precision%29) (InputAction :type Input%20Action%20Object%20Reference :default "/Game/Input/Actions/IA_Reset.IA_Reset"))
  (bind _outactors (Actor|GetAllActorsOfClass "/Game/AI/Path.Path_C"))
  (Transformation|SetActorTransform (Math|Transform|MakeTransform (+ (Spline|FindLocationClosesttoWorldLocation (Variables|/Game/AI/Path.Path_C|GetSpline (Utilities|Array|Get(acopy) _outactors)) (Transformation|GetActorLocation) "World") "0,0,50.000000") (Math|Rotator|MakeRotator 0.0 0.0 (.yaw (Transformation|GetActorRotation)))) false true)
  (Class|PrimitiveComponent|SetPhysicsAngularVelocityinDegrees (Variables|Character|GetMesh) "0, 0, 0" false "None") ; Interrupt any angular movement
  (Physics|SetPhysicsLinearVelocity (Variables|Character|GetMesh) "0, 0, 0" false "None") ; Interrupt any linear movement
)

(event Input|EnhancedActionEvents|EnhancedInputActionIA_Steering
  (params (ActionValue :type Float%20%28double-precision%29) (ElapsedSeconds :type Float%20%28double-precision%29) (TriggeredSeconds :type Float%20%28double-precision%29) (InputAction :type Input%20Action%20Object%20Reference :default "/Game/Input/Actions/IA_Steering.IA_Steering"))
  (bind _vehiclemovementcomponent (Variables|Default|GetVehicleMovementComponent))
  (:Triggered
    (Class|ChaosVehicleMovementComponent|SetSteeringInput _vehiclemovementcomponent ActionValue))
  (:Completed
    (Class|ChaosVehicleMovementComponent|SetSteeringInput _vehiclemovementcomponent ActionValue)))

(event Input|EnhancedActionEvents|EnhancedInputActionIA_Pause
  (params (ActionValue :type Boolean) (ElapsedSeconds :type Float%20%28double-precision%29) (TriggeredSeconds :type Float%20%28double-precision%29) (InputAction :type Input%20Action%20Object%20Reference :default "/Game/Input/Actions/IA_Pause.IA_Pause"))
  (bind _returnvalue (Game|GetPlayerController 0))
  (:Started
    (Game|SetGamePaused true)
    (bind _returnvalue_2 (UserInterface|CreateWidget "/Game/UI/Race/WBP_PauseMenu.WBP_PauseMenu_C" _returnvalue))
    (UserInterface|Viewport|AddtoViewport _returnvalue_2 0)
    (Input|SetInputModeUIOnly _returnvalue _returnvalue_2 "DoNotLock" false)
    (Variables|/Script/Engine.PlayerController|SetbShowMouseCursor _returnvalue true)))

(event Input|EnhancedActionEvents|EnhancedInputActionIA_LookBack
  (params (ActionValue :type Boolean) (ElapsedSeconds :type Float%20%28double-precision%29) (TriggeredSeconds :type Float%20%28double-precision%29) (InputAction :type Input%20Action%20Object%20Reference :default "/Game/Input/Actions/IA_LookBack.IA_LookBack"))
  (:Triggered
    (Transformation|SetRelativeRotation (Variables|Default|GetSpringArm) "0.000000,180.000000,0.000000" false false))
  (:Completed
    (Transformation|SetRelativeRotation (Variables|Default|GetSpringArm) "0, 0, 0" false false)))

(event Input|EnhancedActionEvents|EnhancedInputActionIA_GearDown
  (params (ActionValue :type Float%20%28double-precision%29) (ElapsedSeconds :type Float%20%28double-precision%29) (TriggeredSeconds :type Float%20%28double-precision%29) (InputAction :type Input%20Action%20Object%20Reference :default "/Game/Input/Actions/IA_GearDown.IA_GearDown"))
  (bind _chaos_wheeled_vehicle_movement_component (Variables|Default|GetChaos%20Wheeled%20Vehicle%20Movement%20Component))
  (:Started
    (Class|ChaosVehicleMovementComponent|SetTargetGear _chaos_wheeled_vehicle_movement_component (- (Class|ChaosVehicleMovementComponent|GetTargetGear _chaos_wheeled_vehicle_movement_component) 1) true)))

(event EventBeginPlay
  (bind _mesh (Variables|Character|GetMesh))
  (bind _aschaos_wheeled_vehicle_movement_component (Utilities|Casting|CastToChaosWheeledVehicleMovementComponent (Variables|Default|GetVehicleMovementComponent)))
  (Variables|Default|SetChaos%20Wheeled%20Vehicle%20Movement%20Component _aschaos_wheeled_vehicle_movement_component)
  (Variables|Default|SetName "You")
  (bind _asrace_game_instance (Utilities|Casting|CastToRaceGameInstance (Game|GetGameInstance)))
  (bind _returnvalue (Class|RaceGameInstance|GetCarCustomizations _asrace_game_instance "BP_Hachi_Roku_C"))
  (if (not (== (.CarColor (Utilities|Struct|BreakCarCustomizations _returnvalue)) "(R=0.000000,G=0.000000,B=0.000000,A=0.000000)"))
    (bind _returnvalue_2 (Rendering|Material|CreateDynamicMaterialInstance _mesh (Rendering|Material|GetMaterialIndex _mesh "Paint") "/Game/Art/Vehicles/Hachi_Roku/Materials/Paint_Inst.Paint_Inst" "None" :!class /Script/Engine.PrimitiveComponent))
    (Rendering|Material|SetVectorParameterValue _returnvalue_2 "PaintColor" (.CarColor (Utilities|Struct|BreakCarCustomizations _returnvalue)) :!class /Script/Engine.MaterialInstanceDynamic)))

(event EventTick
  (params (DeltaSeconds :type Float%20%28single-precision%29))
  (bind _engine (Variables|Default|GetEngine))
  (Class|PrimitiveComponent|SetAngularDamping (Variables|Character|GetMesh) (Math|Float|SelectFloat 0.0 5.0 (AI|Components|NavMovement|IsMovingonGround (Variables|Default|GetChaos%20Wheeled%20Vehicle%20Movement%20Component)))) ; Damps rotation when in air
  (CallFunction|InterpstoOriginalRotation)
  (Class|FMODAudioComponent|SetParameter (Variables|Default|GetEngine) "RPM" (Class|ChaosWheeledVehicleMovementComponent|GetEngineRotationSpeed (Variables|Default|GetChaos%20Wheeled%20Vehicle%20Movement%20Component)))
  (bind _returnvalue (Class|ChaosVehicleMovementComponent|GetThrottleInput (Variables|Default|GetChaos%20Wheeled%20Vehicle%20Movement%20Component)))
  (Class|FMODAudioComponent|SetVolume _engine 0.3)
  (Class|FMODAudioComponent|SetParameter _engine "Load" (Math|Float|MapRangeClamped _returnvalue 0.0 1.0 -2e+03 2e+03))
  (CallFunction|ChargeNitrous)
  (Camera|SetFieldOfView (Variables|Default|GetCamera) (Math|Float|MapRangeClamped (Class|ChaosVehicleMovementComponent|GetForwardSpeedMPH (Variables|Default|GetChaos%20Wheeled%20Vehicle%20Movement%20Component)) 6e+01 1.6e+02 9e+01 1e+02)))

(fn ConstructionScript)

(fn BrakeLights
  (params (InputPin :type Boolean))
  (bind _returnvalue (Rendering|Material|CreateDynamicMaterialInstance "/Game/Art/Vehicles/Hachi_Roku/Materials/Red_Lights.Red_Lights" "" "None" :!class /Script/Engine.KismetMaterialLibrary))
  (Rendering|Material|SetMaterial (Variables|Character|GetMesh) 3 _returnvalue)
  (if InputPin
    (Rendering|Material|SetScalarParameterValue _returnvalue "BrakeLightPower" 1.0 :!class /Script/Engine.MaterialInstanceDynamic)
    (else
      (Rendering|Material|SetScalarParameterValue _returnvalue "BrakeLightPower" 0.1 :!class /Script/Engine.MaterialInstanceDynamic))))