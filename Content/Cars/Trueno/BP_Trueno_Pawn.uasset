(event Custom|InterpsToOriginalRotation
  (Transformation|SetRelativeRotation (Variables|Default|GetSpringArm) (Math|Rotator|MakeRotator 0.0 0.0 (Math|Interpolation|FInterpTo (.yaw (Variables|/Script/Engine.SceneComponent|GetRelativeRotation (Variables|Default|GetSpringArm))) 0.0 (Utilities|Time|GetWorldDeltaSeconds) 1.0)) false false) ; Reset camera to original angle
)

(event Input|EnhancedActionEvents|EnhancedInputActionIA_Throttle
  (params (ActionValue :type Float%20%28double-precision%29) (ElapsedSeconds :type Float%20%28double-precision%29) (TriggeredSeconds :type Float%20%28double-precision%29) (InputAction :type Input%20Action%20Object%20Reference :default "/Game/Input/Actions/IA_Throttle.IA_Throttle"))
  (bind _vehiclemovementcomponent (Variables|Default|GetVehicleMovementComponent))
  (:Triggered
    (Class|ChaosVehicleMovementComponent|SetThrottleInput _vehiclemovementcomponent ActionValue))
  (:Completed
    (Class|ChaosVehicleMovementComponent|SetThrottleInput _vehiclemovementcomponent ActionValue)))

(event Input|EnhancedActionEvents|EnhancedInputActionIA_Break
  (params (ActionValue :type Float%20%28double-precision%29) (ElapsedSeconds :type Float%20%28double-precision%29) (TriggeredSeconds :type Float%20%28double-precision%29) (InputAction :type Input%20Action%20Object%20Reference :default "/Game/Input/Actions/IA_Break.IA_Break"))
  (bind _vehiclemovementcomponent (Variables|Default|GetVehicleMovementComponent))
  (:Triggered
    (Class|ChaosVehicleMovementComponent|SetBrakeInput _vehiclemovementcomponent ActionValue))
  (:Completed
    (Class|ChaosVehicleMovementComponent|SetBrakeInput _vehiclemovementcomponent 0.0)))

(event Input|EnhancedActionEvents|EnhancedInputActionIA_LookAround
  (params (ActionValue :type Float%20%28double-precision%29) (ElapsedSeconds :type Float%20%28double-precision%29) (TriggeredSeconds :type Float%20%28double-precision%29) (InputAction :type Input%20Action%20Object%20Reference :default "/Game/Input/Actions/IA_LookAround.IA_LookAround"))
  (:Triggered
    (Transformation|AddLocalRotation (Variables|Default|GetSpringArm) (Math|Rotator|MakeRotator 0.0 0.0 ActionValue) false false) ; Rotate camera around the vehicle
  ))

(event Input|EnhancedActionEvents|EnhancedInputActionIA_Steering
  (params (ActionValue :type Float%20%28double-precision%29) (ElapsedSeconds :type Float%20%28double-precision%29) (TriggeredSeconds :type Float%20%28double-precision%29) (InputAction :type Input%20Action%20Object%20Reference :default "/Game/Input/Actions/IA_Steering.IA_Steering"))
  (bind _vehiclemovementcomponent (Variables|Default|GetVehicleMovementComponent))
  (:Triggered
    (Class|ChaosVehicleMovementComponent|SetSteeringInput _vehiclemovementcomponent ActionValue))
  (:Completed
    (Class|ChaosVehicleMovementComponent|SetSteeringInput _vehiclemovementcomponent ActionValue)))

(event EventBeginPlay
  (bind _aschaos_wheeled_vehicle_movement_component (Utilities|Casting|CastToChaosWheeledVehicleMovementComponent (Variables|Default|GetVehicleMovementComponent)))
  (Variables|Default|SetChaos%20Wheeled%20Vehicle%20Movement%20Component _aschaos_wheeled_vehicle_movement_component)
  (Variables|Default|SetName "You"))

(event EventTick
  (params (DeltaSeconds :type Float%20%28single-precision%29))
  (Class|PrimitiveComponent|SetAngularDamping (Variables|Character|GetMesh) (Math|Float|SelectFloat 0.0 3.0 (AI|Components|NavMovement|IsMovingonGround (Variables|Default|GetChaos%20Wheeled%20Vehicle%20Movement%20Component)))) ; Damps rotation when in air
  (CallFunction|InterpstoOriginalRotation))

(fn ConstructionScript)