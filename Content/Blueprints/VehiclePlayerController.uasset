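; Player controller for the racing game that owns the driving HUD and the end-of-race results screen.
; On BeginPlay it adds the default Enhanced Input mapping, creates the vehicle HUD and caches the pawn's vehicle movement component.
; Each Tick pushes speed and gear from that component, plus position, lap, time and best time from the RaceCarPawn, into the HUD.
; EndRace fills a results widget from a passed array and displays it.
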(event Custom|EndRace
  (params (Array :type Array%20of%20S%20Race%20Data%20Structures))
  (bind _returnvalue (UserInterface|CreateWidget "/Game/UI/UI_EndRace.UI_EndRace_C" self))
  (Default|UpdateList _returnvalue Array)
  (UserInterface|Viewport|AddtoViewport _returnvalue 0))

(event EventBeginPlay
  (Input|AddMappingContext (PlayerController|LocalPlayerSubsystems|GetEnhancedInputLocalPlayerSubsystem) "/Game/Input/IMC_Default.IMC_Default" 0 "(bIgnoreAllPressedKeysUntilRelease=True,bForceImmediately=False)") ; Adding the Input Mapping Context needed to trigger the proper Input Actions.
  (bind _returnvalue (UserInterface|CreateWidget "/Game/UI/UI_VehicleHUD.UI_VehicleHUD_C" self))
  (bind _output_get (Variables|Default|SetVehicleHud _returnvalue))
  (UserInterface|Viewport|AddtoViewport _output_get 0)
  (bind _aswheeled_vehicle_pawn (Utilities|Casting|CastToWheeledVehiclePawn (Pawn|GetControlledPawn)))
  (Variables|Default|SetVehicle%20Movement%20Component (Variables|/Script/ChaosVehicles.WheeledVehiclePawn|GetVehicleMovementComponent _aswheeled_vehicle_pawn)))

(event EventTick
  (params (DeltaSeconds :type Float%20%28single-precision%29))
  (Default|UpdateSpeed (Variables|Default|GetVehicleHud) (Vehicle|GetForwardSpeed (Variables|Default|GetVehicle%20Movement%20Component)))
  (Default|UpdateGear (Variables|Default|GetVehicleHud) (Class|ChaosVehicleMovementComponent|GetCurrentGear (Variables|Default|GetVehicle%20Movement%20Component)))
  (bind _asrace_car_pawn (Utilities|Casting|CastToRaceCarPawn (Pawn|GetControlledPawn)))
  (bind _output_get (Variables|Default|SetAs%20Race%20Car%20Pawn _asrace_car_pawn))
  (Default|UpdatePosition (Variables|Default|GetVehicleHud) (Variables|/Script/Handling.RaceCarPawn|GetCurrentPosition _output_get))
  (Default|UpdateLap (Variables|Default|GetVehicleHud) (Variables|/Script/Handling.RaceCarPawn|GetCurrentLap (Variables|Default|GetAs%20Race%20Car%20Pawn)))
  (Default|UpdateTime (Variables|Default|GetVehicleHud) (Variables|/Script/Handling.RaceCarPawn|GetTimeCounter (Variables|Default|GetAs%20Race%20Car%20Pawn)))
  (bind _returnvalue (Class|RaceCarPawn|GetCurrentBestTime (Variables|Default|GetAs%20Race%20Car%20Pawn)))
  (Default|UpdateBest (Variables|Default|GetVehicleHud) _returnvalue))

(fn ConstructionScript)